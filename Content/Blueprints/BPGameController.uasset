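; Game controller actor for what appears to be a shooter, running the session, enemy spawning and score display.
; StartGame spawns and possesses the player ship, makes this actor the view target and opens a Tick-driven spawn gate.
; A randomized Delay paces random-class enemies at sideways offsets, its interval lengthening per spawn up to a cap.
; A trigger culls tracked enemies, and the construction script positions spawn points, trigger and cleaners.
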(event `self.ReceiveBeginPlay`
  ;[1 1 1] Start and END
  (`self.StartGame`))

(event `StartGame`
  (bind _returnvalue (`GameplayStatics.GetPlayerController` 0))
  (bind _playership (`self.PlayerShip`))
  ;[1 1 1] Start and END
  (set `self.bPlayerDead` false)
  (`AudioComponent.Play` (`self.GameAudio`) 0.0)
  (`|ExecutionSequence`
    (:`then_0`
      (set `self.SpawnInterval` 1.0)
      (`self.ResetSpawnEnemies`)
      (bind _returnvalue_2 (`|SpawnActorFromClass` "/Game/Blueprints/BPPlayer.BPPlayer_C" (`SceneComponent.K2_GetComponentToWorld` (`self.PlayerSpawnPoint`)) "Undefined" "OverrideRootScale"))
      (set `self.PlayerShip` _returnvalue_2)
      (`Controller.Possess` _returnvalue _playership)
      (add `self.OnDestroyed` _playership (delegate `PlayerKilled`))
      (`PlayerController.SetViewTargetWithBlend` _returnvalue self 0.0 "VTBlend_Linear" 0.0 true))
    (:`then_1`
      (`/Engine/EditorBlueprintResources/StandardMacros.Gate` true :!via `Open` :!label _label))))

(event `PlayerKilled`
  ;[1 1 1] Start and END
  (set `self.bPlayerDead` true))

(event `QuitGame`
  ;[1 1 1] Start and END
  (`|ExecutionSequence`
    (:`then_0`
      (goto _label :!via `Close`))
    (:`then_1`
      (`self.K2_DestroyActor` (`self.PlayerShip`))
      (`self.PlayCameraShake`)
      (`AudioComponent.Stop` (`self.GameAudio`)))))

(event `PlayCameraShake`
  (`GameplayStatics.PlayWorldCameraShake` null (`self.K2_GetActorLocation`) 0.0 500.0))

(event `self.Trigger.OnComponentBeginOverlap`
  (params (OtherActor :type "Actor Object Reference") (OtherComp :type "PrimitiveComponent Object Reference") (OtherBodyIndex :type Integer) (bFromSweep :type Boolean) (SweepResult :type "HitResult Structure (by ref)"))
  (if (`KismetArrayLibrary.Array_Contains` (`self.SpawnedEnemies`) OtherActor)
    (`self.K2_DestroyActor` OtherActor)))

(event `self.ReceiveTick`
  (params (DeltaSeconds :type "Float (single-precision)"))
  (bind _spawninterval (`self.SpawnInterval`))
  (bind _enemyspawnpoint (`self.EnemySpawnPoint`))
  (bind _maxhozspawnoffset (`self.MaxHozSpawnOffset`))
  (bind _actorarray (`self.ActorArray`))
  (`/Engine/EditorBlueprintResources/StandardMacros.Gate` true :!label _label_2
    (:`Exit`
      (`KismetSystemLibrary.Delay` (`KismetMathLibrary.RandomFloatInRange` _spawninterval (+ _spawninterval 0.1)))
      (bind _returnvalue (`|SpawnActorFromClass` (`KismetArrayLibrary.Array_Get` _actorarray (`KismetMathLibrary.RandomInteger` (`KismetArrayLibrary.Array_Length` _actorarray))) (`KismetMathLibrary.MakeTransform` (+ (`SceneComponent.K2_GetComponentLocation` _enemyspawnpoint) (`KismetMathLibrary.LessLess_VectorRotator` (`KismetMathLibrary.MakeVector` 0.0 (`KismetMathLibrary.RandomFloatInRange` (* _maxhozspawnoffset -1.0) _maxhozspawnoffset)) (`self.K2_GetActorRotation`))) (`SceneComponent.K2_GetComponentRotation` _enemyspawnpoint) (1.0 1.0 1.0)) "Undefined" "OverrideRootScale"))
      (`KismetArrayLibrary.Array_Add` (`self.SpawnedEnemies`) _returnvalue)
      (add `self.OnDestroyed` _returnvalue (delegate `EnemyDestroyed`))
      (set `self.SpawnInterval` (`KismetMathLibrary.FClamp` (+ (`self.SpawnInterval`) 0.3) 0.7 10.0)))))

(event `ScoreEvent`
  (params (Value :type Integer))
  (`self.ControlScore` Value))

(event `ResetSpawnEnemies`
  (goto _label_2 :!via `Open`))

(event `StopSpawningEnemies`
  (bind _spawnedenemies (`self.SpawnedEnemies`))
  (for _array_element _spawnedenemies
    (`self.K2_DestroyActor` _array_element))
  (`KismetArrayLibrary.Array_Clear` _spawnedenemies)
  (goto _label_2 :!via `Close`))

(event `EnemyDestroyed`
  (if (`self.bPlayerDead`)
    (`/Engine/EditorBlueprintResources/StandardMacros.DoOnce` false :!label _label_3
      (:`Completed`
        (`GameplayStatics.PlaySoundAtLocation` "/Game/Blueprints/Audio/Explosion2.Explosion2")
        (goto _label_3 :!via `Reset`)))))

(fn `ControlScore`
  (params (Value :type Integer))
  (bind _output_get (set `self.Score` (+ Value (`self.Score`))))
  (`TextRenderComponent.K2_SetText` (`self.Scoretextnumber`) (`KismetTextLibrary.Conv_IntToText` _output_get)))

(fn `UserConstructionScript`
  (`SceneComponent.K2_SetRelativeLocation` (`self.PlayerSpawnPoint`) (`self.PlayerSpawnLocation`) false false)
  (`SceneComponent.K2_SetRelativeLocation` (`self.EnemySpawnPoint`) (`self.EnemySpawnLocation`) false false)
  (`SceneComponent.K2_SetRelativeLocation` (`self.Trigger`) (`self.TriggerLocation`) false false)
  (`SceneComponent.K2_SetRelativeLocation` (`self.CleanerTop`) (`self.ProjectileCleanTop`) false false)
  (`SceneComponent.K2_SetRelativeLocation` (`self.CleanerLower`) (`self.ProjectileCleanLower`) false false))