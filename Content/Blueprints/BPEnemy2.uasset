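; BPEnemy2 is a patrolling enemy that slides sideways at a random speed and fires projectiles downward at the player.
; A spawn timeline lowers it into place, then Tick moves it with sweep, and hits damage pawns or reverse its direction otherwise.
; A random Delay on Tick throttles firing while the player is within X range.
; At zero health it explodes, awards score through BPGameController and destroys itself.
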(event `self.ReceiveBeginPlay`
  (bind _spawnlocation (`self.SpawnLocation`))
  (bind _returnvalue (+ (`self.Yaw`) 0.0))
  (set `self.Yaw` (* (.yaw (`self.K2_GetActorRotation` (`self.GetInstigator`))) 0.0))
  (set `self.MoveDirection` (`KismetMathLibrary.RandomBool`))
  (set `self.MoveSpeed` (`KismetMathLibrary.RandomFloatInRange` 30.0 100.0))
  (set `self.SpawnLocation` (`self.K2_GetActorLocation`))
  (bind (_direction _entry) (`Timeline|SpawnAnimation`)
    (:`Update`
      (`self.K2_SetActorLocation` (`KismetMathLibrary.VLerp` _spawnlocation (- _spawnlocation (0.0 0.0 60.0)) _entry))
      (`self.SetActorRotation` (`KismetMathLibrary.RLerp` (`KismetMathLibrary.MakeRotator` 0.0 0.0 _returnvalue) (`KismetMathLibrary.MakeRotator` 0.0 0.0 _returnvalue) _entry)))
    (:`Finished`
      (set `self.MoveEnabled` true))))

(event `self.ReceiveTick`
  (params (DeltaSeconds :type "Float (single-precision)"))
  (bind _returnvalue (`GameplayStatics.GetPlayerPawn` 0))
  (if (`self.MoveEnabled`)
    (`self.K2_SetActorLocation` (+ (`self.K2_GetActorLocation`) (* (`KismetMathLibrary.GreaterGreater_VectorRotator` (`KismetMathLibrary.MakeVector` (* (`self.MoveSpeed`) (`KismetMathLibrary.SelectFloat` 1.0 -1.0 (`self.MoveDirection`)))) (`KismetMathLibrary.MakeRotator` 0.0 0.0 (`self.Yaw`))) DeltaSeconds)) true)
    (`/Engine/EditorBlueprintResources/StandardMacros.IsValid` _returnvalue
      (:`Is Valid`
        (`KismetSystemLibrary.Delay` (`KismetMathLibrary.RandomFloatInRange` 0.1 0.6))
        (if (<= (`KismetMathLibrary.VSize` (* (- (`self.K2_GetActorLocation` _returnvalue) (`self.K2_GetActorLocation`)) (1.0 0.0 0.0))) 120.0)
          (`|SpawnActorFromClass` "/Game/Blueprints/BPProjectileEnemy.BPProjectileEnemy_C" (`self.GetTransform`) "Undefined" "OverrideRootScale" null (`KismetMathLibrary.MakeColor` 1.0 0.3 0.05 1.0) (`KismetMathLibrary.MakeVector` 0.0 0.0 -190.0) self))))))

(event `self.ReceiveHit`
  (params (MyComp :type "PrimitiveComponent Object Reference") (Other :type "Actor Object Reference") (OtherComp :type "PrimitiveComponent Object Reference") (bSelfMoved :type Boolean) (HitLocation :type "Vector Structure") (HitNormal :type "Vector Structure") (NormalImpulse :type "Vector Structure") (Hit :type "HitResult Structure (by ref)"))
  (bind _aspawn (cast `Pawn` Other)
    (:`then`
      (`GameplayStatics.ApplyDamage` _aspawn 10.0))
    (:`CastFailed`
      (set `self.MoveDirection` (not (`self.MoveDirection`))))))

(event `self.ReceiveAnyDamage`
  (params (Damage :type "Float (single-precision)") (DamageType :type "DamageType Object Reference") (InstigatedBy :type "Controller Object Reference") (DamageCauser :type "Actor Object Reference"))
  (set `self.Health` (`KismetMathLibrary.FClamp` (- (`self.Health`) Damage) 0.0 100.0))
  (if (<= (`self.Health`) 0.0)
    (`GameplayStatics.SpawnEmitterAtLocation` "/Game/ExampleContent/Input_Examples/Effects/P_Pixel_Explosion.P_Pixel_Explosion" (`self.K2_GetActorLocation`))
    (bind _outactors (`GameplayStatics.GetAllActorsOfClass` "/Game/Blueprints/BPGameController.BPGameController_C"))
    (`/Game/Blueprints/BPGameController.ScoreEvent` (`KismetArrayLibrary.Array_Get` _outactors) 10)
    (`self.K2_DestroyActor`)))

(fn `UserConstructionScript`)