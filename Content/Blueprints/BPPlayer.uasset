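; Player-controlled shooter actor that flies on a horizontal/vertical plane oriented to its starting yaw, firing projectiles and taking damage.
; A spinning, rising spawn timeline unlocks movement on finish.
; Tick eases input into per-axis speeds through Movement, then applies swept moves and yaws with horizontal speed.
; Held fire loops a timer spawning projectiles from left and right muzzles; damage drains clamped health, destroying the actor at zero.
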(event Custom|FireReset
  (CallFunction|PrimaryFire (Variables|Default|GetLeft))
  (CallFunction|PrimaryFire (Variables|Default|GetRight))
  (Audio|PlaySoundatLocation "/Game/Blueprints/Audio/Shoot2.Shoot2" (Transformation|GetActorLocation)))

(event EventBeginPlay
  (Variables|Default|SetYaw (.Yaw (Math|Rotator|BreakRotator (Transformation|GetActorRotation (Game|GetInstigator)))))
  (Variables|Default|SetSpawnLocation (Transformation|GetActorLocation))
  (bind _lerp (Timeline|SpawnAnimation Play)
    (:Update
      (Transformation|SetActorLocation (Math|Vector|Lerp(Vector) (Variables|Default|GetSpawnLocation) (+ (Variables|Default|GetSpawnLocation) "0, 0,60.000000") _lerp) false false)
      (Transformation|SetActorRotation (Math|Rotator|Lerp(Rotator) "0, 0, 0" (Math|Rotator|MakeRotator 0.0 0.0 (+ 7.2e+02 (Variables|Default|GetYaw))) _lerp)))
    (:Finished
      (Variables|Default|SetbMovementEnabled true))))

(event Game|Damage|EventAnyDamage
  (params (Damage :type Float%20%28single-precision%29) (DamageType :type Damage%20Type%20Object%20Reference) (InstigatedBy :type Controller%20Object%20Reference) (DamageCauser :type Actor%20Object%20Reference))
  (Variables|Default|SetHealth (Math|Float|Clamp(Float) (- (Variables|Default|GetHealth) Damage) 0.0 2.5e+02))
  (Variables|Default|SetCurrentSpeed (* (Variables|Default|GetCurrentSpeed) -0.5))
  (if (<= (Variables|Default|GetHealth) 0.0)
    (Audio|PlaySoundatLocation "/Game/Blueprints/Audio/Explosion2.Explosion2" (Transformation|GetActorLocation))
    (Actor|DestroyActor)))

(event EventTick
  (params (DeltaSeconds :type Float%20%28single-precision%29))
  (Variables|Default|SetDeltaSeconds DeltaSeconds)
  (if (Variables|Default|GetbMovementEnabled)
    (bind _returndirection (CallFunction|Movement (Variables|Default|GetHozSpeed) (Input|AxisValues|GetMoveRight)))
    (bind _returndirection_2 (CallFunction|Movement (Variables|Default|GetVertSpeed) (Input|AxisValues|GetMoveForward)))
    (Variables|Default|SetVertSpeed _returndirection_2)
    (Variables|Default|SetHozSpeed _returndirection)
    (Transformation|SetActorLocation (+ (Transformation|GetActorLocation) (Math|Vector|RotateVector (Math|Vector|MakeVector (stale _output_get) 0.0 (stale _output_get)) (Math|Rotator|MakeRotator 0.0 0.0 (Variables|Default|GetYaw)))) true false)
    (Transformation|SetActorRotation (Math|Interpolation|RInterpTo (Transformation|GetActorRotation) (Math|Rotator|MakeRotator 0.0 0.0 (+ (* (Variables|Default|GetHozSpeed) -1e+01) (Variables|Default|GetYaw))) (Variables|Default|GetDeltaSeconds) 0.0))))

(event Input|ActionEvents|InputActionPrimaryFire
  (params (Key :type Key%20Structure :default "AnyKey"))
  (:Pressed
    (bind _returnvalue (Utilities|Time|SetTimerbyFunctionName 0 "FireReset" 0.2 true))
    (Variables|Default|SetTimeHandle _returnvalue)
    (CallFunction|PrimaryFire (Variables|Default|GetLeft))
    (CallFunction|PrimaryFire (Variables|Default|GetRight))
    (Audio|PlaySoundatLocation "/Game/Blueprints/Audio/Shoot2.Shoot2" (Transformation|GetActorLocation)))
  (:Released
    (Class|KismetSystemLibrary|ClearTimerHandle (Variables|Default|GetTimeHandle))))

(fn ConstructionScript)

(fn Movement
  (params (Speed :type Float%20%28single-precision%29) (Direction :type Float%20%28single-precision%29))
  (bind _output_get (Variables|Default|SetCurrentSpeed (Math|Interpolation|FInterpTo Speed (* (* Direction (Variables|Default|GetMovementSpeed)) (Variables|Default|GetDeltaSeconds)) (Variables|Default|GetDeltaSeconds) 4.0)))
  (return _output_get))

(fn PrimaryFire
  (params (Location :type Scene%20Component%20Object%20Reference))
  (Game|SpawnActorfromClass "/Game/Blueprints/BPProjectile.BPProjectile_C" (Transformation|GetWorldTransform Location) "Undefined" 0 (Math|Color|MakeColor 0.6 0.3 0.6 1.0) (Math|Vector|MakeVector 0.0 0.0 7e+02) self))