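; A coloured projectile actor that flies forward and damages the first actor it touches other than its owner.
; The construction script creates a dynamic material on the Projectile component, which BeginPlay tints with the projectile colour.
; Tick moves the component by a local offset scaled by speed, without sweeping.
; On overlap it applies fixed damage, spawns a pixel explosion emitter and destroys itself.
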(event `self.ReceiveBeginPlay`
  (`MaterialInstanceDynamic.SetVectorParameterValue` (`self.ProjectileMaterial`) "Color2" (`self.ProjectileColour`)))

(event `self.ReceiveTick`
  (params (DeltaSeconds :type "Float (single-precision)"))
  (`SceneComponent.K2_AddLocalOffset` (`self.Projectile`) (* (`self.Speed`) DeltaSeconds) false false))

(event `self.Projectile.OnComponentBeginOverlap`
  (params (OtherActor :type "Actor Object Reference") (OtherComp :type "PrimitiveComponent Object Reference") (OtherBodyIndex :type Integer) (bFromSweep :type Boolean) (SweepResult :type "HitResult Structure (by ref)"))
  (if (!= OtherActor (`self.ProjectileOwner`))
    (`GameplayStatics.ApplyDamage` OtherActor 20.0)
    (`GameplayStatics.SpawnEmitterAtLocation` "/Game/ExampleContent/Input_Examples/Effects/P_Pixel_Explosion.P_Pixel_Explosion" (`self.K2_GetActorLocation`))
    (`self.K2_DestroyActor`)))

(fn `UserConstructionScript`
  (bind _returnvalue (`PrimitiveComponent.CreateDynamicMaterialInstance` (`self.Projectile`) 0 null))
  (set `self.ProjectileMaterial` _returnvalue))